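; Room actor blueprint that shows a paper sprite for an environment room and tracks the interactible objects inside it.
; On BeginPlay it gathers every InteractibleObject in the level whose WhereObject matches its WhereRoom into AllObjectOfRoom.
; The construction script applies the configured sprite and initial visibility, and a SetVisibilityOfObject event toggles the room sprite's visibility at runtime.
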(event EventBeginPlay
  (bind _outactors (Actor|GetAllActorsOfClass "/Game/Blueprint/Environnement/InteractibleObject.InteractibleObject_C"))
  (for _array_element _outactors
    (if (Utilities|Enum|Equal(Enum) (Variables|/Game/Blueprint/Environnement/InteractibleObject.InteractibleObject_C|GetWhere_Object _array_element) (Variables|Default|GetWhere_Room))
      (Utilities|Array|Add (Variables|Default|GetAllObjectOfRoom) _array_element))))

(event EventSetVisibilityOfObject
  (params (SetNewVisibility :type Boolean))
  (bind _papersprite (Variables|Default|GetPaperSprite))
  ;[1 1 1] Set visibility
  (if SetNewVisibility
    (Rendering|SetVisibility _papersprite true false)
    (else
      (Rendering|SetVisibility _papersprite false false))))

(fn ConstructionScript
  (bind _papersprite (Variables|Default|GetPaperSprite))
  ;[1 1 1] Set sprite model
  (Rendering|Components|Sprite|SetSprite (Variables|Default|GetPaperSprite) (Variables|Default|GetSprite))
  (if (Variables|Default|GetVisibility)
    (Rendering|SetVisibility _papersprite true false)
    (else
      (Rendering|SetVisibility _papersprite false false))))