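; Interactible environment object shown as a Paper2D sprite, with configurable sprite and initial visibility applied at construction.
; Hovering the cursor over the sprite toggles the player character's action message, while the Box reports overlap begin and end to the other actor.
; SetVisibilityOfObject switches sprite visibility and collision together, so hidden sprites have no collision.
; TeleportObject moves only the sprite component to the world origin.
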(event OnBeginCursorOver(PaperSprite)
  (params (TouchedComponent :type Primitive%20Component%20Object%20Reference))
  (Class|Communicator|SetAction(Message) (Game|GetPlayerCharacter 0) true self))

(event OnEndCursorOver(PaperSprite)
  (params (TouchedComponent :type Primitive%20Component%20Object%20Reference))
  (Class|Communicator|SetAction(Message) (Game|GetPlayerCharacter 0) false))

(event OnComponentBeginOverlap(Box)
  (params (OverlappedComponent :type Primitive%20Component%20Object%20Reference) (OtherActor :type Actor%20Object%20Reference) (OtherComp :type Primitive%20Component%20Object%20Reference) (OtherBodyIndex :type Integer) (bFromSweep :type Boolean) (SweepResult :type Hit%20Result%20Structure%20%28by%20ref%29))
  (Class|Communicator|PlayerHitInteractibleObject(Message) OtherActor self))

(event OnComponentEndOverlap(Box)
  (params (OverlappedComponent :type Primitive%20Component%20Object%20Reference) (OtherActor :type Actor%20Object%20Reference) (OtherComp :type Primitive%20Component%20Object%20Reference) (OtherBodyIndex :type Integer))
  (Class|Communicator|PlayerHitInteractibleObject(Message) OtherActor))

(event EventTeleportObject
  (Transformation|SetWorldLocation (Variables|Default|GetPaperSprite) "0, 0, 0" false false))

(event EventSetVisibilityOfObject
  (params (SetNewVisibility :type Boolean))
  (bind _papersprite (Variables|Default|GetPaperSprite))
  ;[1 1 1] Set visibility
  (if SetNewVisibility
    (Rendering|SetVisibility _papersprite true false)
    (Collision|SetCollisionEnabled _papersprite "QueryAndPhysics")
    (else
      (Rendering|SetVisibility _papersprite false false)
      (Collision|SetCollisionEnabled _papersprite "NoCollision"))))

(fn ConstructionScript
  (bind _papersprite (Variables|Default|GetPaperSprite))
  ;[1 1 1] Set sprite model
  (Rendering|Components|Sprite|SetSprite (Variables|Default|GetPaperSprite) (Variables|Default|GetSprite))
  (if (Variables|Default|GetVisibility)
    (Rendering|SetVisibility _papersprite true false)
    (Collision|SetCollisionEnabled _papersprite "QueryAndPhysics")
    (else
      (Rendering|SetVisibility _papersprite false false)
      (Collision|SetCollisionEnabled _papersprite "NoCollision"))))