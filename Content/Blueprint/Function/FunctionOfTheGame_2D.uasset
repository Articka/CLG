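; Function library for 2D sprite movement toward destinations and objects.
; MoveToObject adds X-axis movement input to the actor's Instigator, signed by relative position, and fires ActiveActionMessage once the touched object matches the target.
; The match is a reference comparison; an older sprite-name check is left unconnected.
; SetMoveTo returns movement state for a destination and, depending on direction and facing, flips the sprite via RotateSprite.
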(fn MovetoObject
  (params (ForSelf :type Actor%20Object%20Reference) (ToObject :type Actor%20Object%20Reference) (IsOnObject :type Actor%20Object%20Reference))
  (bind _returnvalue (Transformation|GetActorLocation ToObject))
  (bind _instigator (Variables|/Script/Engine.Actor|GetInstigator ForSelf))
  (bind _x (Math|Vector|BreakVector _returnvalue))
  (bind _returnvalue_2 (Math|Vector|MakeVector _x 0.0 0.0))
  (bind _sameobject (CallFunction|MovetoObjectTestObject ToObject IsOnObject))
  (if _sameobject
    _
    (else
      (if (>= (.X (Math|Vector|BreakVector (Transformation|GetWorldLocation (Variables|/Script/Engine.Actor|GetRootComponent ForSelf)))) (.X (Math|Vector|BreakVector (Transformation|GetActorLocation ToObject))))
        (Pawn|Input|AddMovementInput _instigator _returnvalue_2 -1.0 false)
        (else
          (Pawn|Input|AddMovementInput _instigator _returnvalue_2 1.0 false)))
      (bind _sameobject_2 (CallFunction|MovetoObjectTestObject ToObject IsOnObject))
      (if _sameobject_2
        _
        (else
          (return "0, 0, 0" false false)))))
  (Class|Communicator|ActiveAction(Message) ForSelf)
  (return "0, 0, 0" false true))

(fn MovetoObjectTestObject
  (params (ToObject :type Actor%20Object%20Reference) (IsOnObject :type Actor%20Object%20Reference))
  (if (== ToObject IsOnObject)
    (return true)
    (else
      (return false))))

(fn RotateSprite
  (params (ForSelf :type Paper%20Flipbook%20Component%20Object%20Reference))
  (Transformation|AddLocalRotation ForSelf "0,180.000000, 0" false false)
  (return))

(fn SetMoveto
  (params (Destination :type Vector) (ForSelf :type Actor%20Object%20Reference) (isLeft :type Boolean) (Sprite :type Paper%20Flipbook%20Component%20Object%20Reference))
  (if (> (.X (Math|Vector|BreakVector Destination)) (.x (Transformation|GetActorLocation ForSelf)))
    (if isLeft
      _
      (elif isLeft
        (CallFunction|RotateSprite Sprite :!label _label)
        (return false true false Destination)
        (else
          _)))
    (elif isLeft
      (goto _label)
      (else
        _)))
  (return false true true Destination))